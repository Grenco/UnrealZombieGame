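; BP_RayGun is a ray gun weapon Blueprint that drives its own on-screen HUD.
; On BeginPlay it creates a WBP_RayGunHUD widget, adds it to the viewport and keeps a reference to it.
; Its events push ammo to that widget as a fraction of MaxAmmo and forward notification text, with no firing logic in this graph.
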(event `self.ReceiveBeginPlay`
  (bind _returnvalue (`|CreateWidget` "/Game/UI/WBP_RayGunHUD.WBP_RayGunHUD_C"))
  (`UserWidget.AddToViewport` _returnvalue 0)
  (set `self.WeaponHUD` _returnvalue))

(event `self.UpdateAmmoHUD`
  (params (AmmoCount :type "Float (single-precision)") (ReloadCount :type Integer))
  (`/Game/UI/WBP_RayGunHUD.SetAmmo` (`self.WeaponHUD`) (/ AmmoCount (`self.MaxAmmo`))))

(event `self.UpdateNotificationText`
  (params (Text :type String))
  (`/Game/UI/WBP_RayGunHUD.UpdateNotificationText` (`self.WeaponHUD`) Text))

(fn `UserConstructionScript`)