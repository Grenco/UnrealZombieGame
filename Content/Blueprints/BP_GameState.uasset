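; BP_GameState is a game state Blueprint that surfaces wave state changes on the main HUD.
; BeginPlay creates the WBP_MainHUD widget, adds it to the viewport and keeps a reference to it.
; WaveStateChanged briefly shows the new state's enum name as main text and, when a wave is in progress, also pushes WaveCount to the HUD.
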(event `self.WaveStateChanged`
  (params (NewState :type "EWaveState Enum" :default "WaitingToStart") (OldState :type "EWaveState Enum" :default "WaitingToStart"))
  (set `self.New State` NewState)
  (`/Game/UI/WBP_MainHUD.SetMainText` (`self.MainHUD`) (`|GetEnumeratorNameAsString` NewState) 3.0)
  (if (`|EnumEquality` (`self.New State`) "WaveInProgress")
    (`/Game/UI/WBP_MainHUD.SetWaveCount` (`self.MainHUD`) (`self.WaveCount`))))

(event `self.ReceiveBeginPlay`
  (bind _returnvalue (`|CreateWidget` "/Game/UI/WBP_MainHUD.WBP_MainHUD_C"))
  (`UserWidget.AddToViewport` _returnvalue 0)
  (set `self.MainHUD` _returnvalue))

(fn `UserConstructionScript`)