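; BP_TargetDummy is a target dummy that shows the damage it takes and tips over when its health runs out.
; Point damage draws a short-lived red debug number just above the hit location, while radial damage prints "Oof" and the amount to screen.
; BeginPlay binds to HealthComp's OnHealthChanged, which rotates the skeletal mesh once when health hits zero, guarded by the Alive flag.
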(event `self.ReceivePointDamage`
  (params (Damage :type "Float (single-precision)") (DamageType :type "DamageType Object Reference") (HitLocation :type "Vector Structure") (HitNormal :type "Vector Structure") (HitComponent :type "PrimitiveComponent Object Reference") (BoneName :type Name) (ShotFromDirection :type "Vector Structure") (InstigatedBy :type "Controller Object Reference") (DamageCauser :type "Actor Object Reference") (HitInfo :type "HitResult Structure (by ref)"))
  (`KismetSystemLibrary.DrawDebugString` (+ HitLocation (0.0 0.0 10.0)) (`KismetStringLibrary.Conv_Int64ToString` (`KismetMathLibrary.Round64` Damage)) null (struct :`R` 1.0 :`A` 1.0) 0.5))

(event `self.ReceiveRadialDamage`
  (params (DamageReceived :type "Float (single-precision)") (DamageType :type "DamageType Object Reference") (Origin :type "Vector Structure") (HitInfo :type "HitResult Structure (by ref)") (InstigatedBy :type "Controller Object Reference") (DamageCauser :type "Actor Object Reference"))
  (`KismetSystemLibrary.PrintString` "Oof")
  (`KismetSystemLibrary.PrintString` (`KismetStringLibrary.Conv_DoubleToString` DamageReceived)))

(event `self.ReceiveBeginPlay`
  (add `SHealthComponent.OnHealthChanged` (`self.HealthComp`) (delegate `OnHealthChanged_Event_0`))
  (set `self.bAlive` true))

(event `OnHealthChanged_Event_0`
  (params (HealthComp :type "SHealthComponent Object Reference") (Health :type "Float (double-precision)") (HealthDelta :type "Float (double-precision)") (DamageType :type "DamageType Object Reference") (InstigatedBy :type "Controller Object Reference") (DamageCauser :type "Actor Object Reference"))
  (if (and (<= Health 0.0) (`self.bAlive`))
    (`SceneComponent.K2_SetWorldRotation` (`self.SkeletalMesh`) (struct :`Roll` 90.0) false false)
    (set `self.bAlive` false)))

(fn `UserConstructionScript`)