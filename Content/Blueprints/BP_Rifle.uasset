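; BP_Rifle is a rifle weapon Blueprint whose graph handles only the player's weapon HUD.
; CreateWeaponUI spawns WBP_WeaponHUD, adds it to the viewport and stores it, but only when the rifle's owner is player 0's pawn.
; Ammo and notification events forward values to that widget when it is valid, truncating the ammo count to an integer.
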(event `self.ReceiveBeginPlay`)

(event `self.CreateWeaponUI`
  (if (== (`self.GetOwner`) (`GameplayStatics.GetPlayerPawn` 0))
    (bind _returnvalue (`|CreateWidget` "/Game/UI/WBP_WeaponHUD.WBP_WeaponHUD_C"))
    (`UserWidget.AddToViewport` _returnvalue 0)
    (set `self.WeaponHUD` _returnvalue)))

(event `self.UpdateAmmoHUD`
  (params (AmmoCount :type "Float (single-precision)") (ReloadCount :type Integer))
  (bind _weaponhud (`self.WeaponHUD`))
  (`/Engine/EditorBlueprintResources/StandardMacros.IsValid` _weaponhud
    (:`Is Valid`
      (`/Game/UI/WBP_WeaponHUD.SetAmmo` _weaponhud (`KismetMathLibrary.FTrunc` AmmoCount) ReloadCount))))

(event `self.UpdateNotificationText`
  (params (Text :type String))
  (bind _weaponhud (`self.WeaponHUD`))
  (`/Engine/EditorBlueprintResources/StandardMacros.IsValid` _weaponhud
    (:`Is Valid`
      (`/Game/UI/WBP_WeaponHUD.UpdateNotificationText` _weaponhud Text))))

(fn `UserConstructionScript`)