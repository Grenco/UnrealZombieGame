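; BP_AdvancedAI is an AI-controlled actor that runs the BT_AdvancedAI behavior tree and shares its health with it.
; On BeginPlay it starts the tree on its AI controller, binds to the health component's change event and writes the starting health to the blackboard.
; Each health change updates the Blackboard Health key, so the tree can read the current value.
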(event `self.ReceiveBeginPlay`
  (bind _healthcomp (`self.HealthComp`))
  (bind _returnvalue (`AIBlueprintHelperLibrary.GetAIController` self))
  (bind _returnvalue_2 (`AIBlueprintHelperLibrary.GetBlackboard` _returnvalue))
  (`/Engine/EditorBlueprintResources/StandardMacros.IsValid` _returnvalue
    (:`Is Valid`
      (`AIController.RunBehaviorTree` _returnvalue "/Game/AdvancedAI/BT_AdvancedAI.BT_AdvancedAI")
      (`/Engine/EditorBlueprintResources/StandardMacros.IsValid` _returnvalue_2
        (:`Is Valid`
          (`/Engine/EditorBlueprintResources/StandardMacros.IsValid` _healthcomp
            (:`Is Valid`
              (add `SHealthComponent.OnHealthChanged` _healthcomp (delegate `OnHealthChanged_Event_0`))
              (`BlackboardComponent.SetValueAsFloat` _returnvalue_2 "Health" (`SHealthComponent.Health` (`self.HealthComp`))))))))))

(event `OnHealthChanged_Event_0`
  (params (HealthComp :type "SHealthComponent Object Reference") (Health :type "Float (double-precision)") (HealthDelta :type "Float (double-precision)") (DamageType :type "DamageType Object Reference") (InstigatedBy :type "Controller Object Reference") (DamageCauser :type "Actor Object Reference"))
  (`BlackboardComponent.SetValueAsFloat` (`AIBlueprintHelperLibrary.GetBlackboard` (`AIBlueprintHelperLibrary.GetAIController` self)) "Health" Health))

(fn `UserConstructionScript`)